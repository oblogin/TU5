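; BP_PlayerController is a player controller that spawns timeline-driven cubes and speeds up their animation through key presses.
; E spawns an SM_TimelineCube at a stored transform, with the player pawn as owner and instigator, and saves it as the current Cube.
; The 1 key raises the play rate of that cube's TimelineScale timeline by a fixed step, so only the most recently spawned cube is affected.
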(event Custom|AddTimelineCube
  (bind _returnvalue (Game|Player|GetPlayerPawn 0))
  (bind _returnvalue_2 (Game|SpawnActorfromClass "/Game/Blueprints/Timeline/SM_TimelineCube.SM_TimelineCube_C" (Variables|Default|GetSpawn%20Transform) "AlwaysSpawn" _returnvalue _returnvalue))
  (Variables|Default|SetCube _returnvalue_2))

(event Custom|Speed
  (bind _cube (Variables|Default|GetCube))
  (bind _timelinescale (Variables|/Game/Blueprints/Timeline/SM_TimelineCube.SM_TimelineCube_C|GetTimelineScale _cube))
  (Components|Timeline|SetPlayRate _timelinescale (+ (Components|Animation|GetPlayRate _timelinescale) 1.0)))

(event EventBeginPlay)

(event EventTick
  (params (DeltaSeconds :type Float%20%28single-precision%29)))

(event Input|KeyboardEvents|E
  (params (Key :type Key%20Structure :default "None"))
  (:Pressed
    (CallFunction|AddTimelineCube)))

(event Input|KeyboardEvents|1
  (params (Key :type Key%20Structure :default "None"))
  (:Pressed
    (CallFunction|Speed)))

(fn ConstructionScript)